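; BP_Player is the player-controlled actor that moves through Enhanced Input.
; BeginPlay adds the IMC_Player mapping context to the owning player controller's input subsystem.
; While IA_Move triggers, it offsets its location along its forward and right vectors by MoveSpeed times the input's X and Y.
; Movement sets the location directly, with no sweep for collision and no delta-time scaling.
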(event `EnhancedInput|/Game/Blueprints/Inputs/IA_Move`
  (params (ActionValue :type "Vector2D Structure") (ElapsedSeconds :type "Float (double-precision)") (TriggeredSeconds :type "Float (double-precision)") (InputAction :type "InputAction Object Reference" :default "/Game/Blueprints/Inputs/IA_Move.IA_Move"))
  (:`Triggered`
    (`self.K2_SetActorLocation` (+ (`self.K2_GetActorLocation`) (* (`self.GetActorForwardVector`) (* (`self.MoveSpeed`) ActionValue_X)))) ; 위치 변경
    (`self.K2_SetActorLocation` (+ (`self.K2_GetActorLocation`) (* (`self.GetActorRightVector`) (* (`self.MoveSpeed`) ActionValue_Y)))) ; 위치 변경
  ))

(event `self.ReceiveBeginPlay`
  (bind `_as플레이어_컨트롤러` (cast `PlayerController` (`self.GetController`)))
  (`EnhancedInputSubsystemInterface.AddMappingContext` (pcsubsystem `EnhancedInputLocalPlayerSubsystem` `_as플레이어_컨트롤러`) "/Game/Blueprints/Inputs/IMC_Player.IMC_Player" 0 (struct)))

(fn `UserConstructionScript`)